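; BP_CameraPawn is a camera pawn that turns player input into orbit and back-navigation actions.
; On possession by a player controller, it adds the IMC_Main Enhanced Input mapping context.
; IA_View passes its horizontal and vertical values to Orbit only while the right mouse button is held, and IA_Back calls GoBack.
; Orbit and GoBack are called here but implemented outside this graph.
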(event `self.ReceivePossessed`
  (params (NewController :type "Controller Object Reference"))
  (bind _asplayer_controller (cast `PlayerController` NewController))
  (`EnhancedInputSubsystemInterface.AddMappingContext` (pcsubsystem `EnhancedInputLocalPlayerSubsystem` _asplayer_controller) "/Game/General/Input/IMC_Main.IMC_Main" 0 (struct)))

(event `EnhancedInput|/Game/General/Input/IA_View`
  (params (ActionValue :type "Vector2D Structure") (ElapsedSeconds :type "Float (double-precision)") (TriggeredSeconds :type "Float (double-precision)") (InputAction :type "InputAction Object Reference" :default "/Game/General/Input/IA_View.IA_View"))
  (bind (_x _y) (`KismetMathLibrary.BreakVector2D` ActionValue))
  (:`Triggered`
    (if (`PlayerController.IsInputKeyDown` (`GameplayStatics.GetPlayerController` 0) "RightMouseButton")
      (`self.Orbit` _x _y))))

(event `EnhancedInput|/Game/General/Input/IA_Back`
  (params (ActionValue :type Boolean) (ElapsedSeconds :type "Float (double-precision)") (TriggeredSeconds :type "Float (double-precision)") (InputAction :type "InputAction Object Reference" :default "/Game/General/Input/IA_Back.IA_Back"))
  (:`Triggered`
    (`self.GoBack`)))

(fn `UserConstructionScript`)